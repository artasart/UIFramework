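; Player controller that drives the game's UI through a cached BP_HUD, which it has generate the UI and stack the last panel on BeginPlay.
; Left Alt opens a radial menu with UI-only input and a centered cursor; hiding it restores game input, with no actions wired to the selection.
; UIMode and GameMode events switch input and cursor, while debug keys test splash popups and back navigation.
; Friend and profile panel events are empty stubs.
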(event Custom|HideRadialUI
  ;[1 1 1] Radial
  (Variables|Default|SetbShowMouseCursor false)
  (Default|ShowRadialUI (Variables|/Game/Blueprint/BP_HUD.BP_HUD_C|GetRadialWidget (Variables|Default|GetBP_HUD)) false)
  (Input|SetInputModeGameOnly self true)
  (switch Utilities|FlowControl|Switch|SwitchonEnum_Radial (Variables|/Game/Widget/WDG_Radial.WDG_Radial_C|GetEnum_Radial (Variables|/Game/Blueprint/BP_HUD.BP_HUD_C|GetRadialWidget (Variables|Default|GetBP_HUD)))))

(event Custom|ShowRadialUI
  (bind _returnvalue (Viewport|GetViewportSize))
  (bind _bp_hud (Variables|Default|GetBP_HUD))
  (bind _bp_hud_2 (Variables|Default|GetBP_HUD))
  (bind _radialwidget (Variables|/Game/Blueprint/BP_HUD.BP_HUD_C|GetRadialWidget _bp_hud))
  (bind _radialwidget_2 (Variables|/Game/Blueprint/BP_HUD.BP_HUD_C|GetRadialWidget _bp_hud_2))
  ;[1 1 1] Radial
  (Variables|/Script/UMG.Widget|SetVisibility _radialwidget "Visible")
  (Input|SetInputModeUIOnly self _radialwidget "DoNotLock" true)
  (Class|PlayerController|SetMouseLocation (Math|Float|Truncate (/ (.x _returnvalue) 2.0)) (Math|Float|Truncate (/ (.y _returnvalue) 2.0)))
  (Default|HideSelect _radialwidget_2)
  (Default|ShowRadialUI _radialwidget_2 true))

(event Custom|UIMode
  (params (bResetCursor :type Boolean) (Focus :type Widget%20Object%20Reference))
  (bind _returnvalue (Viewport|GetViewportSize))
  (Input|SetInputModeUIOnly self Focus "DoNotLock" false)
  (if bResetCursor
    (Class|PlayerController|SetMouseLocation self (Math|Float|Truncate (/ (.x _returnvalue) 2.0)) (Math|Float|Truncate (/ (.y _returnvalue) 2.0))))
  (Variables|Default|SetbShowMouseCursor true))

(event Custom|GameMode
  (Input|SetInputModeGameOnly self false)
  (Variables|Default|SetbShowMouseCursor false))

(event Custom|ShowPanelFriend)

(event Custom|ShowPanelProfile)

(event EventBeginPlay
  (|UIInitialize)
  (Default|StackLastPanel (Variables|Default|GetBP_HUD)))

(event Input|KeyboardEvents|DebugKeyB
  (params (Key :type Key%20Structure :default "None") (ActionValue :type Input%20Action%20Value%20Structure))
  ;[1 1 1] Create Message
  (:Pressed
    (Default|StackSplash (Variables|Default|GetBP_HUD) "/Game/Widget/Core/Splash/Splash_LevelUp.Splash_LevelUp_C" false false 2.0)))

(event Input|KeyboardEvents|DebugKeyV
  (params (Key :type Key%20Structure :default "None") (ActionValue :type Input%20Action%20Value%20Structure)))

(event Input|KeyboardEvents|DebugKeyX
  (params (Key :type Key%20Structure :default "None") (ActionValue :type Input%20Action%20Value%20Structure))
  (:Pressed
    (Default|StackSplash (Variables|Default|GetBP_HUD) "/Game/Widget/Core/Splash/Splash_Reward.Splash_Reward_C" false true 1.5)))

(event Input|KeyboardEvents|DebugKeyEscape
  (params (Key :type Key%20Structure :default "None") (ActionValue :type Input%20Action%20Value%20Structure))
  (:Pressed
    (Default|Back (Variables|Default|GetBP_HUD))))

(event Input|KeyboardEvents|LeftAlt
  (params (Key :type Key%20Structure :default "None"))
  ;[1 1 1] Radial
  (:Pressed
    (CallFunction|ShowRadialUI)))

(fn ConstructionScript)